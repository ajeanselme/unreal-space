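; BP_Shadow is a whispering fog hazard that closes in on and slows the player approaching its Box center.
; Outer Fog1 overlap shows the player's Fog component and starts a heartbeat, while exit hides it, fades the sound and restores walk speed.
; Tick derives fog scale, walk speed and heartbeat pitch from distance to the center.
; Inner Fog3 raises FogLevel, halving fog scale, fixing heartbeat pitch and hiding Layer1 and Layer2.
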(event `self.ReceiveBeginPlay`
  (`GameplayStatics.SpawnSoundAttached` "/Game/_Github/Sounds/FogWhispers_Cue.FogWhispers_Cue" (`self.Box`) "None" (0.0 0.0 0.0) (struct) "KeepRelativeOffset" false 1.0 1.0 0.0 null null))

(event `self.ReceiveTick`
  (params (DeltaSeconds :type "Float (single-precision)"))
  (if (> (`self.FogLevel`) 0)
    (bind _asplayer_bp (cast `/Game/_Github/FirstPersonBP/Blueprints/PlayerBP` (`GameplayStatics.GetPlayerCharacter` 0)))
    (bind _returnvalue (`KismetMathLibrary.Vector_Distance` (`SceneComponent.K2_GetComponentLocation` (`self.Box`)) (`SceneComponent.K2_GetComponentLocation` (`Character.Mesh` _asplayer_bp))))
    (bind _returnvalue_2 (/ _returnvalue 50.0))
    (`SceneComponent.SetRelativeScale3D` (`/Game/_Github/FirstPersonBP/Blueprints/PlayerBP.Fog` _asplayer_bp) (`KismetMathLibrary.Conv_DoubleToVector` (/ _returnvalue_2 (`KismetMathLibrary.Conv_IntToDouble` (`self.FogLevel`)))))
    (set `CharacterMovementComponent.MaxWalkSpeed` _returnvalue (`Character.CharacterMovement` _asplayer_bp))
    (if (== (`self.FogLevel`) 2)
      (`AudioComponent.SetPitchMultiplier` (`self.HeartBeat`) 1.7)
      (else
        (`AudioComponent.SetPitchMultiplier` (`self.HeartBeat`) (* (/ 1.0 (/ (`KismetMathLibrary.Sqrt` _returnvalue_2) 2.0)) 1.6))))))

(event `self.Fog1.OnComponentBeginOverlap`
  (params (OverlappedComponent :type "PrimitiveComponent Object Reference") (OtherActor :type "Actor Object Reference") (OtherComp :type "PrimitiveComponent Object Reference") (OtherBodyIndex :type Integer) (bFromSweep :type Boolean) (SweepResult :type "HitResult Structure (by ref)"))
  (set `self.FogLevel` 1)
  (bind _asplayer_bp (cast `/Game/_Github/FirstPersonBP/Blueprints/PlayerBP` OtherActor))
  (`SceneComponent.SetHiddenInGame` (`/Game/_Github/FirstPersonBP/Blueprints/PlayerBP.Fog` _asplayer_bp) false false)
  (bind _returnvalue (`GameplayStatics.SpawnSoundAtLocation` "/Game/_Github/Sounds/heartbeat1_Cue.heartbeat1_Cue" (`self.K2_GetActorLocation` _asplayer_bp) (struct) 1.0 1.0 0.0 null null))
  (set `self.HeartBeat` _returnvalue)
  (set `self.PlayerDefaultWalkSpeed` (`CharacterMovementComponent.MaxWalkSpeed` (`Character.CharacterMovement` _asplayer_bp))))

(event `self.Fog1.OnComponentEndOverlap`
  (params (OverlappedComponent :type "PrimitiveComponent Object Reference") (OtherActor :type "Actor Object Reference") (OtherComp :type "PrimitiveComponent Object Reference") (OtherBodyIndex :type Integer))
  (set `self.FogLevel` 0)
  (bind _asplayer_bp (cast `/Game/_Github/FirstPersonBP/Blueprints/PlayerBP` OtherActor))
  (`SceneComponent.SetHiddenInGame` (`/Game/_Github/FirstPersonBP/Blueprints/PlayerBP.Fog` _asplayer_bp) true false)
  (`AudioComponent.FadeOut` (`self.HeartBeat`) 1.0 0.0 "Linear")
  (set `CharacterMovementComponent.MaxWalkSpeed` (`self.PlayerDefaultWalkSpeed`) (`Character.CharacterMovement` (stale `self.Fog1.OnComponentBeginOverlap` _asplayer_bp))))

(event `self.Fog3.OnComponentBeginOverlap`
  (params (OverlappedComponent :type "PrimitiveComponent Object Reference") (OtherActor :type "Actor Object Reference") (OtherComp :type "PrimitiveComponent Object Reference") (OtherBodyIndex :type Integer) (bFromSweep :type Boolean) (SweepResult :type "HitResult Structure (by ref)"))
  (set `self.FogLevel` 2)
  (`SceneComponent.SetVisibility` (`self.Layer2`) false false)
  (`SceneComponent.SetVisibility` (`self.Layer1`) false false)
  (`AudioComponent.SetPitchMultiplier` (`self.HeartBeat`) 3.0))

(event `self.Fog3.OnComponentEndOverlap`
  (params (OverlappedComponent :type "PrimitiveComponent Object Reference") (OtherActor :type "Actor Object Reference") (OtherComp :type "PrimitiveComponent Object Reference") (OtherBodyIndex :type Integer))
  (set `self.FogLevel` 1)
  (`SceneComponent.SetVisibility` (`self.Layer2`) true false)
  (`SceneComponent.SetVisibility` (`self.Layer1`) true false))

(fn `UserConstructionScript`)