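; One-shot trigger actor that spawns a moving BP_Shadow and flashes a danger warning on screen.
; It fires on any actor overlap when OverlapTrigger is set, or through ActivateBPI, passing forward distance, retreat distance and speed to the shadow before starting its movement.
; If the player pawn is PlayerBP, it disables Box collision, blinks DangerWidget, then destroys itself.
; The other interface functions return only default values.
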(event `self.ReceiveActorBeginOverlap`
  (params (OtherActor :type "Actor Object Reference"))
  (if (`self.OverlapTrigger`)
    (bind _returnvalue (`|SpawnActorFromClass` "/Game/_Github/Shadow/BP_Shadow.BP_Shadow_C" (`self.SpawnTransformation`) "Undefined" "OverrideRootScale" null null :!label _label))
    (set `/Game/_Github/Shadow/BP_Shadow.ForwardDistanceToMove` (`self.ForwardDistance`) _returnvalue)
    (set `/Game/_Github/Shadow/BP_Shadow.RetreatDistanceToMove` (`self.RetreatDistance`) _returnvalue)
    (set `/Game/_Github/Shadow/BP_Shadow.Speed` (`self.Speed`) _returnvalue)
    (`/Game/_Github/Shadow/BP_Shadow.MoveToTarget` _returnvalue)
    (cast `/Game/_Github/FirstPersonBP/Blueprints/PlayerBP` (`GameplayStatics.GetPlayerPawn` 0))
    (`PrimitiveComponent.SetCollisionEnabled` (`self.Box`) "NoCollision")
    (bind _returnvalue_2 (`|CreateWidget` "/Game/_Github/Widgets/DangerWidget.DangerWidget_C"))
    (bind _output_get (set `self.DangerWidget` _returnvalue_2))
    (`UserWidget.AddToViewport` _output_get 0)
    (`|PlayAnimation` _output_get (`/Game/_Github/Widgets/DangerWidget.TextBlink` _returnvalue_2) 0.0 3
      (:`Finished`
        (`Widget.RemoveFromParent` (`self.DangerWidget`))
        (`self.K2_DestroyActor`)))))

(event `/Game/AdvancedPuzzleConstructor/BluePrints/Core/BPI_Actor_Action.Activate_BPI`
  (goto _label))

(fn `GetAngularDamping_BPI`
  (returns (AngularDamping :type "Float (double-precision)"))
  (return 0.0))

(fn `GetBoxColorAndState_BPI`
  (returns (BoxType :type "/Game/AdvancedPuzzleConstructor/BluePrints/Core/E_PushBoxType Enum") (InAir :type Boolean) (InCustomState :type Boolean) (IsAttachedToPlayer :type Boolean))
  (return "NewEnumerator1" false false false))

(fn `GetBoxTransform_BPI`
  (returns (BoxTransform :type "Transform Structure"))
  (return))

(fn `GetDeployTime_BPI`
  (returns (DeployTime :type "Float (double-precision)"))
  (return 0.0))

(fn `GetGrabbingData_BPI`
  (returns (GrabVector :type "Vector Structure") (GrabSpeed :type "Float (double-precision)") (ThrowPower :type "Float (double-precision)") (EnableGravityAfterThrow :type Boolean))
  (return (0.0 0.0 0.0) 0.0 0.0 false))

(fn `GetObjectAxis_BPI`
  (returns (Forward :type "Vector Structure") (Right :type "Vector Structure") (Up :type "Vector Structure"))
  (return (0.0 0.0 0.0) (0.0 0.0 0.0) (0.0 0.0 0.0)))

(fn `GetObjectType_BPI`
  (returns (ObjectType :type "/Game/AdvancedPuzzleConstructor/BluePrints/Core/E_OverlappedObjectType Enum"))
  (return "NewEnumerator1"))

(fn `GetPushBoxData_BPI`
  (returns (BoxAngle :type "Float (double-precision)") (HandL :type "Transform Structure") (HandR :type "Transform Structure"))
  (return 0.0))

(fn `GetTargetTransform`
  (returns (Transform :type "Transform Structure"))
  (return))

(fn `GetVoltageCapacity_BPI`
  (returns (CurrentVoltage :type "Float (double-precision)") (MaxVoltage :type "Float (double-precision)"))
  (return 0.0 0.0))

(fn `IsActorActivated_BPI`
  (returns (Activated :type Boolean))
  (return false))

(fn `IsAttachedToConveyor_BPI`
  (returns (Attached :type Boolean))
  (return false))

(fn `IsDeploymentInProgress_BPI`
  (returns (InDeployment :type Boolean))
  (return false))

(fn `IsObjectGrabbed_BPI`
  (returns (Grabbed :type Boolean))
  (return false))

(fn `IsObjectInPickupArea_BPI`
  (returns (InPickupArea :type Boolean))
  (return false))

(fn `IsObjectTeleportable_BPI`
  (returns (Teleportable :type Boolean))
  (return false))

(fn `IsObjectTransportable_BPI`
  (returns (Transportable :type Boolean))
  (return false))

(fn `IsTelekinesisCompatible_BPI`
  (returns (IsTelekinesisObject :type Boolean))
  (return false))

(fn `IsTelekinesisPickupable_BPI`
  (returns (Pickupable :type Boolean))
  (return false))

(fn `ObjectCanBeUsed`
  (returns (Result :type Boolean))
  (return false))

(fn `UserConstructionScript`)