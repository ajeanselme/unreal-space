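; Usable keypad actor that unlocks and opens its target door actors when the player enters the correct code.
; It creates a Keypad widget on BeginPlay, binds its code-entered event, and on use shows it with UI-only input.
; CheckCode handles closing and compares entries to Code.
; Success plays a sound, restores game input, opens the targets and destroys the keypad, while failure briefly shows WRONG and resets entry.
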(event `self.ReceiveBeginPlay`
  (`parent.ReceiveBeginPlay`)
  (bind _returnvalue (`|CreateWidget` "/Game/_Github/Widgets/Keypad.Keypad_C"))
  (bind _output_get (set `self.KeypadWidget` _returnvalue))
  (set `/Game/_Github/Widgets/Keypad.CorrectCode` (`self.Code`) _output_get)
  (add `/Game/_Github/Widgets/Keypad.CodeEntered` _output_get (`|CreateDelegate` :!event `Check Code`)))

(event `CodeResult`
  (params (Success :type Boolean))
  (bind _returnvalue (`GameplayStatics.GetPlayerController` 0))
  (bind _targetactors (`self.TargetActors`))
  (bind _keypadwidget (`self.KeypadWidget`))
  (bind _codetext (`/Game/_Github/Widgets/Keypad.CodeText` _keypadwidget))
  (if Success
    ;[1 1 1] Success
    (`TextBlock.SetText` (`/Game/_Github/Widgets/Keypad.CodeText` _keypadwidget) (`KismetTextLibrary.Conv_StringToText` "SUCCESS"))
    (set `/Game/_Github/Widgets/Keypad.Paused` true _keypadwidget)
    (`GameplayStatics.PlaySound2D` "/Game/_Github/Sounds/keypad_success.keypad_success" 1.0 1.0 0.0 null null)
    (`KismetSystemLibrary.Delay` 1.0)
    (`Widget.RemoveFromParent` (`self.KeypadWidget`))
    (set `PlayerController.bShowMouseCursor` false _returnvalue)
    (`WidgetBlueprintLibrary.SetInputMode_GameOnly` _returnvalue)
    (set `/Game/_Github/Blueprints/Doors/UsuableActivatedDoor.CanOpen` true _targetactors)
    (`/Game/_Github/Blueprints/Doors/UsuableActivatedDoor.OpenDoor` _targetactors)
    (`self.K2_DestroyActor`)
    (else
      ;[1 1 1] Failed
      (set `/Game/_Github/Widgets/Keypad.Paused` true _keypadwidget)
      (set `/Game/_Github/Widgets/Keypad.CurrentCode` "" _keypadwidget)
      (`TextBlock.SetText` _codetext (`KismetTextLibrary.Conv_StringToText` "WRONG"))
      (`GameplayStatics.PlaySound2D` "/Game/_Github/Sounds/keypad_wrong.keypad_wrong" 1.0 1.0 0.0 null null)
      (`KismetSystemLibrary.Delay` 1.0)
      (`TextBlock.SetText` _codetext "")
      (set `/Game/_Github/Widgets/Keypad.Paused` false _keypadwidget))))

(event `ClosePad`
  (bind _returnvalue (`GameplayStatics.GetPlayerController` 0))
  (`Widget.RemoveFromParent` (`self.KeypadWidget`))
  (set `PlayerController.bShowMouseCursor` false _returnvalue)
  (`WidgetBlueprintLibrary.SetInputMode_GameOnly` _returnvalue))

(fn `Check Code`
  (params (CodeEntered :type String) (Keypad :type "/Game/_Github/Widgets/Keypad Object Reference"))
  (if (`KismetStringLibrary.EqualEqual_StrStr` CodeEntered "close")
    (`self.ClosePad`))
  (if (`KismetStringLibrary.EqualEqual_StrStr` CodeEntered (`self.Code`))
    (`self.CodeResult` true)
    (else
      (`self.CodeResult` false))))

(fn `UseItem`
  (bind _returnvalue (`GameplayStatics.GetPlayerController` 0))
  (bind _keypadwidget (`self.KeypadWidget`))
  (`parent.UseItem`)
  (`UserWidget.AddToViewport` _keypadwidget 0)
  (set `PlayerController.bShowMouseCursor` true _returnvalue)
  (`WidgetBlueprintLibrary.SetInputMode_UIOnlyEx` _returnvalue _keypadwidget))

(fn `UserConstructionScript`
  (`parent.UserConstructionScript`))