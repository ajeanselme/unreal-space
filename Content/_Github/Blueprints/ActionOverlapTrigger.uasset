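; Trigger volume actor that fires configured actions on target actors when something overlaps its box.
; On overlap it walks the TargetActors array and passes each actor and action pair to LIBExecuteAction.
; An AlreadyUsed flag makes it one-shot once any action runs, and an empty array prints a warning with the actor's name.
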(event `self.Box.OnComponentBeginOverlap`
  (params (OverlappedComponent :type "PrimitiveComponent Object Reference") (OtherActor :type "Actor Object Reference") (OtherComp :type "PrimitiveComponent Object Reference") (OtherBodyIndex :type Integer) (bFromSweep :type Boolean) (SweepResult :type "HitResult Structure (by ref)"))
  (if (`self.AlreadyUsed`)
    _
    (elif (> (`KismetArrayLibrary.Array_Length` (`self.TargetActors`)) 0)
      (for _array_element (`self.TargetActors`)
        (bind (_actor _action) (break `/Game/AdvancedPuzzleConstructor/BluePrints/Core/F_ButtonSimpleAction` _array_element))
        (`/Game/AdvancedPuzzleConstructor/BluePrints/Core/APC_Library.LIB_ExecuteAction` _actor _action)
        (set `self.AlreadyUsed` true))
      (else
        (`KismetSystemLibrary.PrintString` (`KismetStringLibrary.Concat_StrStr` (`KismetSystemLibrary.GetDisplayName` self) ": TargetActors is empty!") true true (struct :`R` 1.0 :`G` 0.160801 :`A` 1.0) 3.0)))))

(fn `UserConstructionScript`)