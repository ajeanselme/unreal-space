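; A usable card reader that unlocks and opens a linked door when the player uses it with a card equipped.
; UseItem checks that the player's equipped item is a PickableItem_Card, then sets the linked DoorToActivate to openable and opens it.
; The card is removed from the player and the reader destroys itself, making it a single-use interaction.
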(fn `UseItem`
  (bind _doortoactivate (`self.DoorToActivate`))
  (`parent.UseItem`)
  (bind _asplayer_bp (cast `/Game/_Github/FirstPersonBP/Blueprints/PlayerBP` (`GameplayStatics.GetPlayerCharacter` 0)))
  (cast `/Game/_Github/Blueprints/PickableItem_Card` (`/Game/_Github/FirstPersonBP/Blueprints/PlayerBP.ItemEquipped` _asplayer_bp))
  (set `/Game/_Github/Blueprints/Doors/UsuableActivatedDoor.CanOpen` true _doortoactivate)
  (`/Game/_Github/Blueprints/Doors/UsuableActivatedDoor.OpenDoor` _doortoactivate)
  (`/Game/_Github/FirstPersonBP/Blueprints/PlayerBP.RemoveEquipedItem` _asplayer_bp)
  (`self.K2_DestroyActor`))

(fn `UserConstructionScript`
  (`parent.UserConstructionScript`))