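; Box-activated puzzle plate whose ButtonType sets its mesh, material, sounds and which boxes it accepts.
; A looping timer polls for overlaps, detaches a suitable box from the player and glides it into place with a timeline.
; Placement and removal trigger configured actions on TargetActors through interface messages and a shared library.
; Paused-until-needed timers charge the box on charger plates or drain its voltage into connected actors, with blinker and audio feedback.
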(event `self.ReceiveBeginPlay`
  ;[1 0.7655 0.1745] Begin Play init
  (`self.InitAudio`)
  (set `self.PowerConnected` false)
  (bind _returnvalue (`KismetSystemLibrary.K2_SetTimer` null "CheckBoxOverlap" 0.2 true))
  (bind _output_get (set `self.CheckBoxPlacedTimeHandle` _returnvalue))
  (`KismetSystemLibrary.K2_UnPauseTimerHandle` _output_get)
  (bind _returnvalue_2 (`KismetSystemLibrary.K2_SetTimer` null "ConnectPowerToActor" 0.5 true))
  (bind _output_get_2 (set `self.ConnectPowerTimeHandler` _returnvalue_2))
  (`KismetSystemLibrary.K2_PauseTimerHandle` _output_get_2)
  (bind _returnvalue_3 (`KismetSystemLibrary.K2_SetTimer` null "ChargePower" 1.0 true))
  (bind _output_get_3 (set `self.ChargePowerTimeHandler` _returnvalue_3))
  (`KismetSystemLibrary.K2_PauseTimerHandle` _output_get_3)
  (set `self.IsBoxPlaced` false)
  (bind _returnvalue_4 (`PrimitiveComponent.CreateDynamicMaterialInstance` (`self.ButtonMesh`) 0 "/Game/AdvancedPuzzleConstructor/Materials/M_Blinker.M_Blinker" "None"))
  (bind _output_get_4 (set `self.BlinkerMat` _returnvalue_4))
  (`MaterialInstanceDynamic.SetVectorParameterValue` _output_get_4 "TestColor" (`self.DisabledColor`)))

(event `ManageSound`
  (params (StartSound :type Boolean))
  ;[1 1 1] Sound manager. Play different sound based on Box type
  (switch `/Game/AdvancedPuzzleConstructor/BluePrints/Core/E_ButtonBoxType` (`self.ButtonType`)
    (:`NewEnumerator0`
      (if StartSound :!label _label
        (`/Game/AdvancedPuzzleConstructor/BluePrints/Core/APC_AudioComponent.StartToLoop` (`self.APC_AudioComponent`) :!label _label_2)
        (goto _label_3 :!via `Reset`)))
    (:`NewEnumerator1`
      (goto _label))
    (:`NewEnumerator2`
      (goto _label))
    (:`NewEnumerator3`
      (if (and (< (`self.BoxVoltage`) (`self.BoxVoltageCapacity`)) StartSound)
        (goto _label_2)
        (else
          (`/Engine/EditorBlueprintResources/StandardMacros.DoOnce` false :!label _label_3
            (:`Completed`
              (`/Game/AdvancedPuzzleConstructor/BluePrints/Core/APC_AudioComponent.LoopToEnd` (`self.APC_AudioComponent`)))))))
    (:`NewEnumerator5`
      (goto _label))
    (:`NewEnumerator6`
      (goto _label))))

(event `ManageSoundConnect`
  (params (StartSound :type Boolean))
  ;[1 1 1] Sound manager. Play different sound based on Box type
  (if (and (> (`self.BoxVoltage`) 0.0) StartSound)
    (goto _label_2)
    (else
      (goto _label_3))))

(event `CheckBoxOverlap`
  (bind _overlappingactors (`PrimitiveComponent.GetOverlappingActors` (`self.BoxArea`) null))
  (bind _output (`|GetArrayItem` _overlappingactors))
  ;[1 1 1] Time function. Check is any actor is overlapped Box Button
  (if (`self.IsBoxPlaced`)
    (set `self.BoxFound` false)
    (for _array_element (`PrimitiveComponent.GetOverlappingActors` (`self.BoxArea`) null)
      (if (`KismetSystemLibrary.DoesImplementInterface` _array_element "/Game/AdvancedPuzzleConstructor/BluePrints/Core/BPI_ObjectControls.BPI_ObjectControls_C")
        (if (== (`self.BoxActor`) _array_element)
          (set `self.BoxFound` true)
          (break))))
    (if (not (`self.BoxFound`))
      (set `self.IsBoxPlaced` false)
      (`self.ExecuteAction` false)
      (`MaterialInstanceDynamic.SetVectorParameterValue` (`self.BlinkerMat`) "TestColor" (`self.DisabledColor`))
      (`self.ManageSound` false)
      (set `self.PrevConnected` false))
    (elif (and (not (`self.IsBoxPlaced`)) (== (`KismetArrayLibrary.Array_Length` _overlappingactors) 1))
      (if (`KismetSystemLibrary.DoesImplementInterface` _output "/Game/AdvancedPuzzleConstructor/BluePrints/Core/BPI_ObjectControls.BPI_ObjectControls_C")
        (bind _objecttype (message `/Game/AdvancedPuzzleConstructor/BluePrints/Core/BPI_ObjectControls.GetObjectType_BPI` _output))
        (if (`|EnumEquality` _objecttype "NewEnumerator0")
          (bind (_boxtype _inair _incustomstate _isattachedtoplayer) (message `/Game/AdvancedPuzzleConstructor/BluePrints/Core/BPI_ObjectControls.GetBoxColorAndState_BPI` _output))
          (bind _iscorrecttype (`self.CheckBoxSuitableType` _boxtype))
          (if _iscorrecttype
            (set `self.CurrentBoxType` _boxtype)
            (if (and (not _inair) (not _incustomstate))
              (set `self.BoxActor` _output)
              (if _isattachedtoplayer
                (message `/Game/AdvancedPuzzleConstructor/BluePrints/Core/BPI_ObjectControls.DetachFromPlayer_BPI` _output))
              (message `/Game/AdvancedPuzzleConstructor/BluePrints/Core/BPI_ObjectControls.SetCustomState_BPI` _output true)
              (`self.StartTransition`)
              (set `self.IsBoxPlaced` true))))))))

(event `StartTransition`
  (bind _boxactor (`self.BoxActor`))
  (bind _boxactor_2 (`self.BoxActor`))
  (bind _boxactor_3 (`self.BoxActor`))
  ;[1 1 1] Transition box to the target location
  (message `/Game/AdvancedPuzzleConstructor/BluePrints/Core/BPI_ObjectControls.SetCustomState_BPI` _boxactor true)
  (message `/Game/AdvancedPuzzleConstructor/BluePrints/Core/BPI_ObjectControls.HideWidgets_BPI` _boxactor true)
  (bind _boxtransform (message `/Game/AdvancedPuzzleConstructor/BluePrints/Core/BPI_ObjectControls.GetBoxTransform_BPI` _boxactor))
  (set `self.StartBoxLocation` (.location _boxtransform))
  (message `/Game/AdvancedPuzzleConstructor/BluePrints/Core/BPI_ObjectControls.StartTransitionRotation_BPI` _boxactor true false)
  (bind (_direction _newtrack_0) (`Timeline|Transition` :!via `PlayFromStart`)
    (:`Update`
      (message `/Game/AdvancedPuzzleConstructor/BluePrints/Core/BPI_ObjectControls.SetBoxLocation_BPI` _boxactor_2 (`KismetMathLibrary.VLerp` (`self.StartBoxLocation`) (`SceneComponent.K2_GetComponentLocation` (`self.Arrow`)) _newtrack_0))
      (message `/Game/AdvancedPuzzleConstructor/BluePrints/Core/BPI_ObjectControls.UpdateBoxActorLocation_BPI` _boxactor_2))
    (:`Finished`
      (message `/Game/AdvancedPuzzleConstructor/BluePrints/Core/BPI_ObjectControls.SetCustomState_BPI` _boxactor_3 false)
      (message `/Game/AdvancedPuzzleConstructor/BluePrints/Core/BPI_ObjectControls.UpdateWidgets_BPI` _boxactor_3)
      (bind (_currentvoltage _maxvoltage) (message `/Game/AdvancedPuzzleConstructor/BluePrints/Core/BPI_ObjectControls.GetVoltageCapacity_BPI` _boxactor_3))
      (bind _output_get (set `self.BoxVoltage` _currentvoltage))
      (bind _output_get_2 (set `self.BoxVoltageCapacity` _maxvoltage))
      (if (>= _output_get _output_get_2)
        (`MaterialInstanceDynamic.SetVectorParameterValue` (`self.BlinkerMat`) "TestColor" (`self.EnabledColor`))
        (`self.ExecuteAction` true)
        (`self.ManageSound` true)))))

(event `ExecuteAction`
  (params (BoxPlaced :type Boolean))
  (bind _connectpowertimehandler (`self.ConnectPowerTimeHandler`))
  (bind _chargepowertimehandler (`self.ChargePowerTimeHandler`))
  ;[1 1 1] Excute Action
  (if (`|EnumEquality` (`self.ButtonType`) "NewEnumerator3")
    (if BoxPlaced
      (if (`KismetSystemLibrary.K2_IsTimerPausedHandle` _chargepowertimehandler)
        (`KismetSystemLibrary.K2_UnPauseTimerHandle` _chargepowertimehandler))
      (else
        (`KismetSystemLibrary.K2_PauseTimerHandle` _chargepowertimehandler)))
    (elif (> (`KismetArrayLibrary.Array_Length` (`self.TargetActors`)) 0)
      (for _array_element (`self.TargetActors`)
        (bind (_actor _boxyep _boxnop) (break `/Game/AdvancedPuzzleConstructor/BluePrints/Core/F_ButtonBoxAction` _array_element))
        (`/Engine/EditorBlueprintResources/StandardMacros.IsValid` _actor
          (:`Is Valid`
            (if BoxPlaced
              (bind _output_get (set `self.ButtonAction` _boxyep))
              (if (and (`|EnumEquality` _output_get "NewEnumerator2") (`|EnumEquality` (`self.CurrentBoxType`) "NewEnumerator4"))
                (set `self.PowerConnected` true)
                ;;[0 1 0.03046] Connect power
                (message `/Game/AdvancedPuzzleConstructor/BluePrints/Core/BPI_Actor_Action.ReconnectPower_BPI` _actor)
                (else
                  (`/Game/AdvancedPuzzleConstructor/BluePrints/Core/APC_Library.LIB_ExecuteAction` _actor (`self.ButtonAction`) :!label _label_4)))
              (else
                (bind _output_get_2 (set `self.ButtonAction` _boxnop))
                (if (`|EnumEquality` _output_get_2 "NewEnumerator7")
                  ;;[1 0.1326 0.09279] Disconnect power
                  (message `/Game/AdvancedPuzzleConstructor/BluePrints/Core/BPI_Actor_Action.DisconnectPower_BPI` _actor)
                  (set `self.PowerConnected` false)
                  (else
                    (goto _label_4))))))
          (:`Is Not Valid`
            (`KismetSystemLibrary.PrintString` (`KismetStringLibrary.Concat_StrStr` (`KismetSystemLibrary.GetDisplayName` self) ": Actor in TargetActors not specified!") true true (struct :`R` 1.0 :`G` 0.160801 :`A` 1.0) 3.0))))
      (if (`self.PowerConnected`)
        (`KismetSystemLibrary.K2_UnPauseTimerHandle` _connectpowertimehandler)
        (elif (`KismetSystemLibrary.K2_IsTimerActiveHandle` _connectpowertimehandler)
          (`KismetSystemLibrary.K2_PauseTimerHandle` _connectpowertimehandler)))
      (else
        (`KismetSystemLibrary.PrintString` (`KismetStringLibrary.Concat_StrStr` (`KismetSystemLibrary.GetDisplayName` self) ": TargetActors is empty!") true true (struct :`R` 1.0 :`G` 0.160801 :`A` 1.0) 3.0)))))

(event `ConnectPowerToActor`
  (bind _isanyactoractivated (`self.IsAnyActorActivated`))
  (bind _boxactor (`self.BoxActor`))
  ;[1 1 1] Connect Power
  (bind (_currentvoltage _maxvoltage) (message `/Game/AdvancedPuzzleConstructor/BluePrints/Core/BPI_ObjectControls.GetVoltageCapacity_BPI` _boxactor))
  (set `self.IsAnyActorActivated` false)
  (for _array_element (`self.TargetActors`)
    (bind (_actor _boxyep) (break `/Game/AdvancedPuzzleConstructor/BluePrints/Core/F_ButtonBoxAction` _array_element))
    (if (`|EnumEquality` _boxyep "NewEnumerator2")
      (message `/Game/AdvancedPuzzleConstructor/BluePrints/Core/BPI_Actor_Action.ConnectPower_BPI` _actor _currentvoltage _maxvoltage (`self.DischargeSpeed`))
      (bind _activated (message `/Game/AdvancedPuzzleConstructor/BluePrints/Core/BPI_Actor_Action.IsActorActivated_BPI` _actor))
      (set `self.IsAnyActorActivated` (or _activated (`self.IsAnyActorActivated`)))))
  (if (`self.IsAnyActorActivated`)
    (bind _returnvalue (`KismetMathLibrary.FClamp` (- _currentvoltage (`self.DischargeSpeed`)) 0.0 100000.0))
    (message `/Game/AdvancedPuzzleConstructor/BluePrints/Core/BPI_ObjectControls.SetBoxVoltage_BPI` _boxactor _returnvalue))
  (`|ExecutionSequence`
    (:`then_0`
      (if (!= _isanyactoractivated (`self.PrevConnected`))
        (if _isanyactoractivated
          (`self.ManageSoundConnect` true)
          (else
            (`self.ManageSoundConnect` false)))
        (set `self.PrevConnected` _isanyactoractivated)))
    (:`then_1`
      (if (<= _returnvalue 0.0)
        (`self.ManageSoundConnect` false)))))

(event `ChargePower`
  (bind _boxactor (`self.BoxActor`))
  ;[1 1 1] Charging Power Box. Pass voltage value to the Box actor
  (bind (_currentvoltage _maxvoltage) (message `/Game/AdvancedPuzzleConstructor/BluePrints/Core/BPI_ObjectControls.GetVoltageCapacity_BPI` _boxactor))
  (bind _returnvalue (`KismetMathLibrary.FClamp` (+ _currentvoltage (`self.ChargeSpeed`)) 0.0 _maxvoltage))
  (message `/Game/AdvancedPuzzleConstructor/BluePrints/Core/BPI_ObjectControls.SetBoxVoltage_BPI` _boxactor _returnvalue)
  (if (>= _returnvalue _maxvoltage)
    (`self.ManageSound` false)))

(fn `CheckBoxSuitableType`
  (params (PushingBox :type "/Game/AdvancedPuzzleConstructor/BluePrints/Core/E_PushBoxType Enum" :default "NewEnumerator1"))
  (returns (IsCorrectTYpe :type Boolean))
  (locals (` Result` :type Boolean))
  ;[1 1 1] Check if placed box is compatible with Button type
  (switch `/Game/AdvancedPuzzleConstructor/BluePrints/Core/E_ButtonBoxType` (`self.ButtonType`)
    (:`NewEnumerator0`
      (set `local. Result` (`|EnumEquality` PushingBox "NewEnumerator1")))
    (:`NewEnumerator1`
      (set `local. Result` (`|EnumEquality` PushingBox "NewEnumerator2")))
    (:`NewEnumerator2`
      (set `local. Result` (`|EnumEquality` PushingBox "NewEnumerator3")))
    (:`NewEnumerator3`
      (set `local. Result` (`|EnumEquality` PushingBox "NewEnumerator4") :!label _label))
    (:`NewEnumerator4`
      (goto _label))
    (:`NewEnumerator5`
      (set `local. Result` (`|EnumEquality` PushingBox "NewEnumerator5")))
    (:`NewEnumerator6`
      (set `local. Result` true)))
  (return (`local. Result`)))

(fn `InitAudio`
  (bind _apc_audiocomponent (`self.APC_AudioComponent`))
  ;[1 1 1] Set specified sounds for APC audio component
  (switch `/Game/AdvancedPuzzleConstructor/BluePrints/Core/E_ButtonBoxType` (`self.ButtonType`)
    (:`NewEnumerator0`
      (`/Game/AdvancedPuzzleConstructor/BluePrints/Core/APC_AudioComponent.Init` _apc_audiocomponent "/Game/AdvancedPuzzleConstructor/Sounds/Cue/BoxPlaced_Cue.BoxPlaced_Cue" null null 1.0 :!label _label))
    (:`NewEnumerator1`
      (goto _label))
    (:`NewEnumerator2`
      (goto _label))
    (:`NewEnumerator3`
      (`/Game/AdvancedPuzzleConstructor/BluePrints/Core/APC_AudioComponent.Init` _apc_audiocomponent "/Game/AdvancedPuzzleConstructor/Sounds/Cue/ChargerStart_Cue.ChargerStart_Cue" "/Game/AdvancedPuzzleConstructor/Sounds/Cue/ChargerEnd_Cue.ChargerEnd_Cue" "/Game/AdvancedPuzzleConstructor/Sounds/Cue/ChargerLoop_Cue.ChargerLoop_Cue" 1.0))
    (:`NewEnumerator4`
      (`/Game/AdvancedPuzzleConstructor/BluePrints/Core/APC_AudioComponent.Init` _apc_audiocomponent "/Game/AdvancedPuzzleConstructor/Sounds/Cue/PowerBoxStart_Cue.PowerBoxStart_Cue" "/Game/AdvancedPuzzleConstructor/Sounds/Cue/PowerBoxEnd_Cue.PowerBoxEnd_Cue" "/Game/AdvancedPuzzleConstructor/Sounds/Cue/PowerBoxLoop_Cue.PowerBoxLoop_Cue" 1.0))
    (:`NewEnumerator5`
      (goto _label))
    (:`NewEnumerator6`
      (goto _label))))

(fn `IsActorActivated_BPI`
  (returns (Activated :type Boolean))
  ;[1 1 1] Return Default value
  (return false))

(fn `SetButtonSkin`
  (locals (TempMat :type "MaterialInstance Object Reference"))
  (bind _buttonmesh (`self.ButtonMesh`))
  (bind _buttonmesh_2 (`self.ButtonMesh`))
  (bind _buttonmesh_3 (`self.ButtonMesh`))
  (bind _buttonmesh_4 (`self.ButtonMesh`))
  (bind _buttonmesh_5 (`self.ButtonMesh`))
  ;[1 1 1] Set meshes for Button based on button type
  (switch `/Game/AdvancedPuzzleConstructor/BluePrints/Core/E_ButtonBoxType` (`self.ButtonType`)
    (:`NewEnumerator0`
      (set `local.TempMat` (`self.GreenMaterial`))
      (`StaticMeshComponent.SetStaticMesh` _buttonmesh_5 "/Game/AdvancedPuzzleConstructor/Meshes/SM_ButtonBox.SM_ButtonBox" :!label _label)
      (`PrimitiveComponent.SetMaterial` _buttonmesh_5 0 "/Game/AdvancedPuzzleConstructor/Materials/M_Blinker.M_Blinker")
      (`PrimitiveComponent.SetMaterial` _buttonmesh_5 1 (`local.TempMat`)))
    (:`NewEnumerator1`
      (set `local.TempMat` (`self.RedMaterial`))
      (goto _label))
    (:`NewEnumerator2`
      (set `local.TempMat` (`self.BlueMaterial`))
      (goto _label))
    (:`NewEnumerator3`
      (`StaticMeshComponent.SetStaticMesh` _buttonmesh "/Game/AdvancedPuzzleConstructor/Meshes/SM_ButtonBoxElectricCharger.SM_ButtonBoxElectricCharger")
      (`PrimitiveComponent.SetMaterial` _buttonmesh 0 "/Game/AdvancedPuzzleConstructor/Materials/M_Blinker.M_Blinker")
      (`PrimitiveComponent.SetMaterial` _buttonmesh 1 (`self.ElectricMaterial`)))
    (:`NewEnumerator4`
      (`StaticMeshComponent.SetStaticMesh` _buttonmesh_3 "/Game/AdvancedPuzzleConstructor/Meshes/SM_ButtonBoxElectricDischarger.SM_ButtonBoxElectricDischarger")
      (`PrimitiveComponent.SetMaterial` _buttonmesh_3 0 "/Game/AdvancedPuzzleConstructor/Materials/M_Blinker.M_Blinker")
      (`PrimitiveComponent.SetMaterial` _buttonmesh_3 1 (`self.DischargerMaterial`)))
    (:`NewEnumerator5`
      (`StaticMeshComponent.SetStaticMesh` _buttonmesh_4 "/Game/AdvancedPuzzleConstructor/Meshes/SM_ButtonBox.SM_ButtonBox")
      (`PrimitiveComponent.SetMaterial` _buttonmesh_4 0 "/Game/AdvancedPuzzleConstructor/Materials/M_Blinker.M_Blinker")
      (`PrimitiveComponent.SetMaterial` _buttonmesh_4 1 (`self.FragileMaterial`)))
    (:`NewEnumerator6`
      (`StaticMeshComponent.SetStaticMesh` _buttonmesh_2 "/Game/AdvancedPuzzleConstructor/Meshes/SM_ButtonBox.SM_ButtonBox")
      (`PrimitiveComponent.SetMaterial` _buttonmesh_2 0 "/Game/AdvancedPuzzleConstructor/Materials/M_Blinker.M_Blinker")
      (`PrimitiveComponent.SetMaterial` _buttonmesh_2 1 (`self.AllMaterial`)))))

(fn `UserConstructionScript`
  (`self.SetButtonSkin`))