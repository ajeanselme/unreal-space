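; Usable post-it panel actor that UseItem toggles the player into and out of.
; Entering teleports the player to PlayerPos at their current height, zeroes walk speed after caching it, fixes camera rotation, and enables the cursor with Game-and-UI input.
; Exiting calls DropPostit on PlayerBP, restores walk speed, controller-driven rotation and game-only input.
; An ExitKeyPanel widget, created at BeginPlay, shows while the panel is in use.
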(event `self.ReceiveBeginPlay`
  (`parent.ReceiveBeginPlay`)
  (bind _returnvalue (`|CreateWidget` "/Game/_Github/Widgets/ExitKeyPanel.ExitKeyPanel_C"))
  (set `self.ExitHUD` _returnvalue))

(fn `UseItem`
  (bind _returnvalue (`GameplayStatics.GetPlayerController` 0))
  (bind _returnvalue_2 (`GameplayStatics.GetPlayerCharacter` 0))
  (bind _returnvalue_3 (`GameplayStatics.GetPlayerController` 0))
  (if (`self.IsBeingUsed`)
    (set `self.IsBeingUsed` false)
    (set `PlayerController.bShowMouseCursor` false _returnvalue_3)
    (`WidgetBlueprintLibrary.SetInputMode_GameOnly` _returnvalue_3)
    (bind _asplayer_bp (cast `/Game/_Github/FirstPersonBP/Blueprints/PlayerBP` (`GameplayStatics.GetPlayerCharacter` 0)))
    (`/Game/_Github/FirstPersonBP/Blueprints/PlayerBP.DropPostit` _asplayer_bp)
    (set `CharacterMovementComponent.MaxWalkSpeed` (`self.maxSpeed`) (`Character.CharacterMovement` _asplayer_bp))
    (set `/Game/_Github/FirstPersonBP/Blueprints/PlayerBP.IsInPostitPanel` false _asplayer_bp)
    (set `Pawn.bUseControllerRotationYaw` true _asplayer_bp)
    (set `CameraComponent.bUsePawnControlRotation` true (`/Game/_Github/FirstPersonBP/Blueprints/PlayerBP.FollowCamera` _asplayer_bp))
    (`Widget.RemoveFromParent` (`self.ExitHUD`))
    (else
      (set `self.IsBeingUsed` true)
      (`parent.UseItem`)
      (set `PlayerController.bShowMouseCursor` true _returnvalue)
      (`WidgetBlueprintLibrary.SetInputMode_GameAndUIEx` _returnvalue null)
      (bind _asplayer_bp_2 (cast `/Game/_Github/FirstPersonBP/Blueprints/PlayerBP` _returnvalue_2))
      (bind _charactermovement (`Character.CharacterMovement` _asplayer_bp_2))
      (set `self.maxSpeed` (`CharacterMovementComponent.MaxWalkSpeed` _charactermovement))
      (set `CharacterMovementComponent.MaxWalkSpeed` 0.0 _charactermovement)
      (set `/Game/_Github/FirstPersonBP/Blueprints/PlayerBP.IsInPostitPanel` true _asplayer_bp_2)
      (`CharacterMovementComponent.ClearAccumulatedForces` _charactermovement)
      (set `Pawn.bUseControllerRotationYaw` false _asplayer_bp_2)
      (bind _followcamera (`/Game/_Github/FirstPersonBP/Blueprints/PlayerBP.FollowCamera` _asplayer_bp_2))
      (set `CameraComponent.bUsePawnControlRotation` false _followcamera)
      (`SceneComponent.K2_SetWorldRotation` _followcamera (struct :`Yaw` 90.0) false false)
      (`UserWidget.AddToViewport` (`self.ExitHUD`) 0)
      (`self.K2_SetActorLocation` _returnvalue_2 (`KismetMathLibrary.MakeVector` (.x (`SceneComponent.K2_GetComponentLocation` (`self.PlayerPos`))) (.y (`SceneComponent.K2_GetComponentLocation` (`self.PlayerPos`))) (.z (`self.K2_GetActorLocation` _returnvalue_2))) false true))))

(fn `UserConstructionScript`
  (`parent.UserConstructionScript`))